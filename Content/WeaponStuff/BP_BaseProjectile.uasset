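; Base projectile actor that explodes when its capsule hits something, dealing area damage and then destroying itself.
; Each hit applies two stacked damage passes at the impact point: flat radial damage, then falloff damage reaching out to a multiplied outer radius with a quarter of base damage as minimum.
; PlayImpactEffects spawns an explosion emitter at the hit location, sized by EmitterScale.
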(event OnComponentHit(Capsule)
  (params (HitComponent :type Primitive%20Component%20Object%20Reference) (OtherActor :type Actor%20Object%20Reference) (OtherComp :type Primitive%20Component%20Object%20Reference) (NormalImpulse :type Vector :default "0, 0, 0") (Hit :type Hit%20Result%20Structure%20%28by%20ref%29))
  (bind _location (Collision|BreakHitResult Hit))
  (bind _damageradius (Variables|Default|GetDamageRadius))
  (bind _basedamage (Variables|Default|GetBaseDamage))
  ;[1 1 1] Apply Damage on Hitting actors
  (Game|Damage|ApplyRadialDamage (Variables|Default|GetBaseDamage) _location (Variables|Default|GetDamageRadius) 0 0 self (Game|GetInstigatorController) false "ECC_Visibility")
  (CallFunction|PlayImpactEffects (Math|Transform|MakeTransform _location "0, 0, 0" "1,1,1"))
  (Class|GameplayStatics|ApplyRadialDamagewithFalloff _basedamage (/ _basedamage 4.0) _location _damageradius (* _damageradius (Variables|Default|GetDamageRadiusMultiplier)) (Variables|Default|GetDamageFalloff) 0 0 self (Game|GetInstigatorController) "ECC_Visibility")
  (Actor|DestroyActor))

(fn ConstructionScript)

(fn PlayImpactEffects
  (params (HitLocation :type Transform))
  (Effects|SpawnEmitteratLocation "/Game/WeaponStuff/FXVarietyPack/Particles/P_ky_explosion.P_ky_explosion" (.location HitLocation) "0, 0, 0" (Variables|Default|GetEmitterScale)))