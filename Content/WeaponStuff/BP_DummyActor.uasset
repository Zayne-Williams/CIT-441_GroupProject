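; BP_DummyActor is a damage test dummy that displays its Health as text through a TextRender component.
; BeginPlay writes the starting Health to the text, and AnyDamage recalculates and redisplays it.
; The recalculation sets Health to Damage minus Health, the reverse of a usual subtraction.
; The check for Health at or below zero runs the same text update on both branches, so no death handling exists.
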(event Game|Damage|EventAnyDamage
  (params (Damage :type Float%20%28single-precision%29) (DamageType :type Damage%20Type%20Object%20Reference) (InstigatedBy :type Controller%20Object%20Reference) (DamageCauser :type Actor%20Object%20Reference))
  (bind _textrender (Variables|Default|GetTextRender))
  (bind _output_get (Variables|Default|SetHealth (- Damage (Variables|Default|GetHealth))))
  (if (<= _output_get 0.0)
    (Rendering|Components|TextRender|SetText _textrender (Utilities|Text|ToText(Float) (Variables|Default|GetHealth) "HalfToEven"))
    (else
      (Rendering|Components|TextRender|SetText _textrender (Utilities|Text|ToText(Float) (Variables|Default|GetHealth) "HalfToEven")))))

(event EventBeginPlay
  (Rendering|Components|TextRender|SetText (Variables|Default|GetTextRender) (Utilities|Text|ToText(Float) (Variables|Default|GetHealth) "HalfToEven")))

(fn ConstructionScript)