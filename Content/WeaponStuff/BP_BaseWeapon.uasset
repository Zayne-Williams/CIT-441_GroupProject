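; Base weapon Blueprint that tracks magazine ammo and handles firing and reloading.
; It sets its skeletal mesh at construction and fills ammo at BeginPlay.
; Fire only checks and decrements ammo and reports success, with effects in a separate animation function.
; Reload draws on MainCharacter reserves by AmmoType, but its clamp zeroes the reserve, and Pistol and Shotgun reload to zero.
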(event EventBeginPlay
  (Variables|Default|SetRemainingAmmo (Variables|Default|GetMaxAmmo)))

(fn ConstructionScript
  (Class|SkinnedMeshComponent|SetSkeletalMesh (Variables|Default|GetGunMesh) (Variables|Default|GetBaseWeaponMesh) true))

(fn CanWeaponFire
  (if (> (Variables|Default|GetRemainingAmmo) 0)
    (return true)
    (else
      (return false))))

(fn Fire
  (params (CrosshairWorldSpace :type Vector))
  (bind _canfire (CallFunction|CanWeaponFire))
  (if _canfire
    (Variables|Default|SetCanFire true)
    (CallFunction|DecrementAmmo)
    (Variables|Default|SetSuccess true)
    (else
      (Variables|Default|SetCanFire false)
      (Variables|Default|SetSuccess false))))

(fn Reload
  (bind _asmain_character (Utilities|Casting|CastToMainCharacter (Game|Player|GetPlayerPawn 0)))
  (switch name (Variables|Default|GetAmmoType)
    (:Rifle
      (bind _output_get (Variables|Default|SetRemainingAmmo (Math|Integer|Clamp(Integer) (Variables|/Game/Blueprints/MainCharacter.MainCharacter_C|GetRifleAmmo _asmain_character) 0 (Variables|Default|GetMaxAmmo))))
      (Variables|/Game/Blueprints/MainCharacter.MainCharacter_C|SetRifleAmmo _asmain_character (Math|Integer|Clamp(Integer) (- (Variables|/Game/Blueprints/MainCharacter.MainCharacter_C|GetRifleAmmo _asmain_character) _output_get) 0 0))
      (Development|PrintString "Rifle"))
    (:Rocket
      (bind _output_get_2 (Variables|Default|SetRemainingAmmo (Math|Integer|Clamp(Integer) (Variables|/Game/Blueprints/MainCharacter.MainCharacter_C|GetRocketAmmo _asmain_character) 0 (Variables|Default|GetMaxAmmo))))
      (Variables|/Game/Blueprints/MainCharacter.MainCharacter_C|SetRocketAmmo _asmain_character (Math|Integer|Clamp(Integer) (- (Variables|/Game/Blueprints/MainCharacter.MainCharacter_C|GetRocketAmmo _asmain_character) _output_get_2) 0 0))
      (Development|PrintString "Rocket"))
    (:Grenade
      (bind _output_get_3 (Variables|Default|SetRemainingAmmo (Math|Integer|Clamp(Integer) (Variables|/Game/Blueprints/MainCharacter.MainCharacter_C|GetGrenadeAmmo _asmain_character) 0 (Variables|Default|GetMaxAmmo))))
      (Variables|/Game/Blueprints/MainCharacter.MainCharacter_C|SetGrenadeAmmo _asmain_character (Math|Integer|Clamp(Integer) (- (Variables|/Game/Blueprints/MainCharacter.MainCharacter_C|GetGrenadeAmmo _asmain_character) _output_get_3) 0 0))
      (Development|PrintString "Grenade"))
    (:Pistol
      (bind _output_get_4 (Variables|Default|SetRemainingAmmo 0))
      (Variables|/Game/Blueprints/MainCharacter.MainCharacter_C|SetPistolAmmo _asmain_character (Math|Integer|Clamp(Integer) (- (Variables|/Game/Blueprints/MainCharacter.MainCharacter_C|GetPistolAmmo _asmain_character) _output_get_4) 0 0))
      (Development|PrintString "Pistol"))
    (:Shotgun
      (bind _output_get_5 (Variables|Default|SetRemainingAmmo 0))
      (Variables|/Game/Blueprints/MainCharacter.MainCharacter_C|SetShotgunAmmo _asmain_character (Math|Integer|Clamp(Integer) (- (Variables|/Game/Blueprints/MainCharacter.MainCharacter_C|GetShotgunAmmo _asmain_character) _output_get_5) 0 0))
      (Development|PrintString "Shotgun"))))

(fn PlaySuccessEffects
  (Components|Animation|PlayAnimation (Variables|Default|GetGunMesh) 0 false))

(fn DecrementAmmo
  (bind _output_get (Variables|Default|SetRemainingAmmo (Math|Integer|Clamp(Integer) (- (Variables|Default|GetRemainingAmmo) 1) 0 (Variables|Default|GetMaxAmmo))))
  (Development|PrintString (Utilities|String|ToString(Integer) _output_get)))