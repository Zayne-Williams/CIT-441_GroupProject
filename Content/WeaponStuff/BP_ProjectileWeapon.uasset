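; Base-style projectile weapon Blueprint that spawns a configurable projectile when fired.
; Fire runs the parent logic first, then calls FireProjectile if CanFire is true.
; The projectile spawns just ahead of the gun mesh's Muzzle socket, owned by the weapon.
; Its rotation comes from player 0's base aim rotation, rather than the muzzle or the passed crosshair position.
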(event EventFire
  (params (CrosshairWorldSpace :type Vector :default "0, 0, 0"))
  (|CallParentFunction CrosshairWorldSpace)
  (if (Variables|Default|GetCanFire)
    (CallFunction|FireProjectile)))

(fn ConstructionScript
  (|CallParentFunction))

(fn FireProjectile
  (bind _gunmesh (Variables|Default|GetGunMesh))
  (bind _muzzle (Variables|Default|GetMuzzle))
  (Game|SpawnActorfromClass (Variables|Default|GetProjectileToLaunch) (Math|Transform|MakeTransform (+ (Transformation|GetSocketLocation _gunmesh _muzzle) (Math|Rotator|GetRotationXVector (Transformation|GetSocketRotation _gunmesh _muzzle))) (Pawn|GetBaseAimRotation (Game|Player|GetPlayerPawn 0))) "Undefined" self (Game|GetInstigator)))