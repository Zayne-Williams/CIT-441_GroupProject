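; BP_Pistol is a pistol weapon Blueprint that layers pistol-specific animations onto a parent weapon class.
; Fire runs the parent logic and plays the pistol fire animation on GunMesh only when Success is true.
; Reload calls the parent and always plays the pistol reload animation.
; A hit on GunMesh from a MainCharacter sets the pistol as that character's CurrentWeapon, acting as a simple pickup.
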(event OnComponentHit(GunMesh)
  (params (HitComponent :type Primitive%20Component%20Object%20Reference) (OtherActor :type Actor%20Object%20Reference) (OtherComp :type Primitive%20Component%20Object%20Reference) (NormalImpulse :type Vector :default "0, 0, 0") (Hit :type Hit%20Result%20Structure%20%28by%20ref%29))
  (bind _asmain_character (Utilities|Casting|CastToMainCharacter OtherActor))
  (Variables|/Game/Blueprints/MainCharacter.MainCharacter_C|SetCurrentWeapon _asmain_character self))

(event EventFire
  (params (CrosshairWorldSpace :type Vector :default "0, 0, 0"))
  (|CallParentFunction CrosshairWorldSpace)
  (if (Variables|Default|GetSuccess)
    (Components|Animation|PlayAnimation (Variables|Default|GetGunMesh) "/Game/WeaponStuff/SciFiWeapDark/Weapons/Anims/Fire_Pistol_W.Fire_Pistol_W" false)))

(event EventReload
  (|CallParentFunction)
  (Components|Animation|PlayAnimation (Variables|Default|GetGunMesh) "/Game/WeaponStuff/SciFiWeapDark/Weapons/Anims/Reload_Pistol_W.Reload_Pistol_W" false))

(fn ConstructionScript
  (|CallParentFunction))