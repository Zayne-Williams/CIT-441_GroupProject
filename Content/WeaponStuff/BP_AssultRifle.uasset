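; BP_AssultRifle is an assault rifle weapon Blueprint that specializes a parent weapon class with rifle-specific animations.
; Fire calls the parent and plays the rifle fire animation only on success, while Reload calls the parent and always plays the hip reload animation.
; When a MainCharacter overlaps the gun mesh, the rifle sets itself as that character's CurrentWeapon.
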(event OnComponentBeginOverlap(GunMesh)
  (params (OverlappedComponent :type Primitive%20Component%20Object%20Reference) (OtherActor :type Actor%20Object%20Reference) (OtherComp :type Primitive%20Component%20Object%20Reference) (OtherBodyIndex :type Integer) (bFromSweep :type Boolean) (SweepResult :type Hit%20Result%20Structure%20%28by%20ref%29))
  (bind _asmain_character (Utilities|Casting|CastToMainCharacter OtherActor))
  (Variables|/Game/Blueprints/MainCharacter.MainCharacter_C|SetCurrentWeapon _asmain_character self))

(event EventFire
  (params (CrosshairWorldSpace :type Vector :default "0, 0, 0"))
  (|CallParentFunction CrosshairWorldSpace)
  (if (Variables|Default|GetSuccess)
    (Components|Animation|PlayAnimation (Variables|Default|GetGunMesh) "/Game/WeaponStuff/SciFiWeapDark/Weapons/Anims/Fire_Rifle_W.Fire_Rifle_W" false)))

(event EventReload
  (|CallParentFunction)
  (Components|Animation|PlayAnimation (Variables|Default|GetGunMesh) "/Game/WeaponStuff/SciFiWeapDark/Weapons/Anims/Reload_Rifle_Hip_W.Reload_Rifle_Hip_W" false))

(fn ConstructionScript
  (|CallParentFunction))