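; Hitscan weapon Blueprint that extends its parent's Fire event with instant line-trace hits and point damage.
; FindHitObject casts one Visibility trace per projectile from the muzzle socket, randomized within a spread cone aimed at the crosshair's world point, with persistent debug drawing.
; DamageHitActors then damages each recorded hit's actor, taking direction from hit toward instigator pawn but always passing the first hit as HitInfo.
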(event EventFire
  (params (CrosshairWorldSpace :type Vector :default "0, 0, 0"))
  (|CallParentFunction CrosshairWorldSpace)
  (bind _hit_ (CallFunction|FindHitObject CrosshairWorldSpace))
  (if _hit_
    (CallFunction|DamageHitActors)))

(fn ConstructionScript
  (|CallParentFunction))

(fn FindHitObject
  (params (CrosshairWorldSpace :type Vector))
  (bind _muzzelsocket (Variables|Default|GetMuzzelSocket))
  (bind _gunmesh (Variables|Default|GetGunMesh))
  (bind _returnvalue (Transformation|GetSocketTransform _gunmesh _muzzelsocket "RTS_World"))
  (Utilities|Array|Clear (Variables|Default|GetHitResults))
  (for _index (range 1 (Variables|Default|GetProjectilesFired))
    (bind (_outhit _returnvalue_2) (Collision|LineTraceByChannel (.location _returnvalue) (+ (.location _returnvalue) (Math|Vector|RotateVector (* (Class|KismetMathLibrary|RandomUnitVectorinConeinRadians "1.000000, 0, 0" (Math|Trig|DegreesToRadians (Variables|Default|GetSpread))) (Variables|Default|GetRange)) (Math|Rotator|FindLookatRotation (.location _returnvalue) CrosshairWorldSpace))) "TraceTypeQuery1" false 0 "Persistent"))
    (bind _output_get (LocalVariables|SetObjectHit? (or _returnvalue_2 (LocalVariables|GetObjectHit?))))
    (if _output_get
      (Utilities|Array|Add (Variables|Default|GetHitResults) _outhit)))
  (return (LocalVariables|GetObjectHit?)))

(fn DamageHitActors
  (bind _hitresults (Variables|Default|GetHitResults))
  (for _index (range 0 (- (Utilities|Array|Length (Variables|Default|GetHitResults)) 1))
    (Game|Damage|ApplyPointDamage (.hitactor (Utilities|Array|Get(acopy) _hitresults _index)) (Variables|Default|GetBaseDamage) (Math|Rotator|GetRotationXVector (Math|Rotator|FindLookatRotation (.location (Utilities|Array|Get(acopy) _hitresults _index)) (Transformation|GetActorLocation (Pawn|GetControlledPawn (Game|GetInstigatorController))))) (Utilities|Array|Get(acopy) _hitresults) 0 self)))