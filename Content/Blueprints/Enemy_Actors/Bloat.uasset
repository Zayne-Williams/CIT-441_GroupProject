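; Bloat is an enemy pawn that damages the main character on overlap and spawns three Leach actors when killed.
; Tick checks squared distance against AgroRange, then either pursues and faces the player or wanders.
; Wandering moves to random reachable points around its spawn, with randomized timer pauses.
; Damage tints a dynamic material from white toward red, though the handler overwrites HP with the HP/MaxHP ratio on each hit.
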(event EventBeginPlay
  (bind _returnvalue (Transformation|GetActorLocation))
  (Variables|Default|SetTargetPoint _returnvalue)
  (Variables|Default|SetWanderCenter _returnvalue)
  (bind _returnvalue_2 (Rendering|Material|CreateDynamicMaterialInstance "/Game/Blueprints/Enemy_Actors/Enemy_Textures/Bloat/PumpkinHulk_Material.PumpkinHulk_Material" "None" :!class /Script/Engine.KismetMaterialLibrary))
  (bind _output_get (Variables|Default|SetDynamMaterial _returnvalue_2))
  (Rendering|Material|SetMaterial (Variables|Default|GetSkeletalMesh) 0 _output_get))

(event Collision|EventActorBeginOverlap
  (params (OtherActor :type Actor%20Object%20Reference))
  (bind _asmain_character (Utilities|Casting|CastToMainCharacter OtherActor))
  (Default|DecrementHealth _asmain_character (Variables|Default|GetDMG)))

(event EventTick
  (params (DeltaSeconds :type Float%20%28single-precision%29))
  (bind _floatingpawnmovement (Variables|Default|GetFloatingPawnMovement))
  (bind _velocity (Variables|/Script/Engine.MovementComponent|GetVelocity _floatingpawnmovement))
  (CallFunction|CheckforPlayerinRange)
  (if (Variables|Default|GetIsInRange)
    (Utilities|FlowControl|Sequence
      (:then_0
        (CallFunction|PersuePlayer))
      (:then_1
        (Transformation|SetActorRotation (Math|Rotator|MakeRotator 0.0 0.0 (.yaw (Math|Rotator|MakeRotfromX (- (Transformation|GetActorLocation (Game|Player|GetPlayerPawn 0)) (Transformation|GetActorLocation))))))))
    (else
      (Utilities|FlowControl|Sequence
        (:then_0
          (CallFunction|WanderAround true "0, 0, 0"))
        (:then_1
          (if (> (Math|Vector|VectorLengthSquared _velocity) 0.1)
            (Transformation|SetActorRotation (Math|Rotator|MakeRotator 0.0 0.0 (.yaw (Math|Rotator|MakeRotfromX _velocity))))))))))

(event Game|Damage|EventAnyDamage
  (params (Damage :type Float%20%28single-precision%29) (DamageType :type Damage%20Type%20Object%20Reference) (InstigatedBy :type Controller%20Object%20Reference) (DamageCauser :type Actor%20Object%20Reference))
  (bind _output_get (Variables|Default|SetHP (- (Variables|Default|GetHP) Damage)))
  (bind _output_get_2 (Variables|Default|Set%25HP (/ _output_get (Variables|Default|GetMax%20HP))))
  (Rendering|Material|SetVectorParameterValue (Variables|Default|GetDynamMaterial) "Color" (Math|Color|Lerp(LinearColor) "(R=1.000000,G=0.000000,B=0.000000,A=1.000000)" "(R=1.000000,G=1.000000,B=1.000000,A=1.000000)" _output_get_2) :!class /Script/Engine.MaterialInstanceDynamic)
  (if (<= _output_get 0.0)
    (Game|SpawnActorfromClass "/Game/Blueprints/Enemy_Actors/Leach.Leach_C" (Math|Transform|MakeTransform (Transformation|GetWorldLocation (Variables|Default|GetLeachSpawn1)) "0, 0, 0" "1,1,1") "AlwaysSpawn" 0 0)
    (Game|SpawnActorfromClass "/Game/Blueprints/Enemy_Actors/Leach.Leach_C" (Math|Transform|MakeTransform (Transformation|GetWorldLocation (Variables|Default|GetLeachSpawn2)) "0, 0, 0" "1,1,1") "AlwaysSpawn" 0 0)
    (Game|SpawnActorfromClass "/Game/Blueprints/Enemy_Actors/Leach.Leach_C" (Math|Transform|MakeTransform (Transformation|GetWorldLocation (Variables|Default|GetLeachSpawn3)) "0, 0, 0" "1,1,1") "AlwaysSpawn" 0 0)
    (Actor|DestroyActor)))

(fn ConstructionScript)

(fn CheckforPlayerinRange
  (if (<= (Class|KismetMathLibrary|VectorDistanceSquared (Transformation|GetActorLocation) (Transformation|GetActorLocation (Game|Player|GetPlayerPawn 0))) (Variables|Default|GetAgroRange))
    (Variables|Default|SetIsInRange true)
    (else
      (Variables|Default|SetIsInRange false))))

(fn PersuePlayer
  (AI|Navigation|SimpleMovetoActor (Pawn|GetController) (Game|Player|GetPlayerPawn 0)))

(fn WanderAround
  (params (UseRandPoint :type Boolean) (Point :type Vector))
  (if (Variables|Default|GetCanWander)
    (if (<= (Math|Vector|Distance(Vector) (Transformation|GetActorLocation) (Variables|Default|GetTargetPoint)) 1.7e+02)
      (Variables|Default|SetCanWander false)
      (Utilities|Time|SetTimerbyFunctionName 0 "SetCanWander" (Math|Random|RandomFloatinRange 1.5 4.0))
      (if UseRandPoint
        (bind _output_get (Variables|Default|SetTargetPoint (.RandomLocation (AI|Navigation|GetRandomReachablePointinRadius (Variables|Default|GetWanderCenter) (Variables|Default|GetWanderRadius) 0 0))))
        (AI|Navigation|SimpleMovetoLocation (Pawn|GetController) _output_get)))))

(fn SetCanWander
  (Variables|Default|SetCanWander true))