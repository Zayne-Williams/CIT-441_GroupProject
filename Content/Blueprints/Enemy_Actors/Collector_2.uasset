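; Collector_2 is an enemy pawn that wanders around its start point until the player enters aggro range.
; Each Tick, squared-distance checks choose between timer-paced navmesh wandering, direct XY-offset pursuit, and attacking, with yaw following velocity or player.
; In attack range it spawns a single ConeAttack_2 at component W, destroying it when pursuit resumes.
; SearchAndDestroy duplicates the chase-or-fire logic but is never called here.
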(event EventBeginPlay
  (bind _returnvalue (Transformation|GetActorLocation))
  (Variables|Default|SetTargetPoint _returnvalue)
  (Variables|Default|SetWanderCenter _returnvalue))

(event Collision|EventActorBeginOverlap
  (params (OtherActor :type Actor%20Object%20Reference)))

(event EventTick
  (params (DeltaSeconds :type Float%20%28single-precision%29))
  (bind _floatingpawnmovement (Variables|Default|GetFloatingPawnMovement))
  (bind _velocity (Variables|/Script/Engine.MovementComponent|GetVelocity _floatingpawnmovement))
  (CallFunction|CheckforPlayerinRange)
  (if (Variables|Default|GetIsInRange)
    (CallFunction|InAttackRange)
    (Utilities|FlowControl|Sequence
      (:then_0
        (if (Variables|Default|GetAttacking)
          (CallFunction|Attack)
          (else
            (CallFunction|PersuePlayer)
            (Variables|Default|SetIsFiring false)
            (Actor|DestroyActor (Variables|Default|GetCurrentCone)))))
      (:then_1
        (Transformation|SetActorRotation (Math|Rotator|MakeRotator 0.0 0.0 (.yaw (Math|Rotator|MakeRotfromX (- (Transformation|GetActorLocation (Game|Player|GetPlayerPawn 0)) (Transformation|GetActorLocation))))))))
    (else
      (Utilities|FlowControl|Sequence
        (:then_0
          (CallFunction|WanderAround true "0, 0, 0"))
        (:then_1
          (if (> (Math|Vector|VectorLengthSquared _velocity) 0.1)
            (Transformation|SetActorRotation (Math|Rotator|MakeRotator 0.0 0.0 (.yaw (Math|Rotator|MakeRotfromX _velocity))))))))))

(fn ConstructionScript)

(fn CheckforPlayerinRange
  (if (<= (Class|KismetMathLibrary|VectorDistanceSquared (Transformation|GetActorLocation) (Transformation|GetActorLocation (Game|Player|GetPlayerPawn 0))) (Variables|Default|GetAgroRange))
    (Variables|Default|SetIsInRange true)
    (else
      (Variables|Default|SetIsInRange false))))

(fn PersuePlayer
  (bind _returnvalue (Utilities|Time|GetWorldDeltaSeconds))
  (bind _returnvalue_2 (Game|Player|GetPlayerPawn 0))
  (bind _returnvalue_3 (Transformation|GetActorLocation))
  (bind _movespeed (Variables|Default|GetMoveSpeed))
  (bind _returnvalue_4 (Transformation|GetActorLocation _returnvalue_2))
  (bind _returnvalue_5 (* _movespeed _returnvalue))
  (bind _returnvalue_6 (- _returnvalue_4 _returnvalue_3))
  (bind _returnvalue_7 (Math|Vector|Normalize _returnvalue_6))
  (bind _returnvalue_8 (* _returnvalue_7 _returnvalue_5))
  (Transformation|AddActorWorldOffset (Math|Vector|MakeVector (.x _returnvalue_8) (.y _returnvalue_8) 0.0)))

(fn WanderAround
  (params (UseRandPoint :type Boolean) (Point :type Vector))
  (if (Variables|Default|GetCanWander)
    (if (<= (Math|Vector|Distance(Vector) (Transformation|GetActorLocation) (Variables|Default|GetTargetPoint)) 1.7e+02)
      (Variables|Default|SetCanWander false)
      (Utilities|Time|SetTimerbyFunctionName 0 "SetCanWander" (Math|Random|RandomFloatinRange 1.5 4.0))
      (if UseRandPoint
        (bind _output_get (Variables|Default|SetTargetPoint (.RandomLocation (AI|Navigation|GetRandomReachablePointinRadius (Variables|Default|GetWanderCenter) (Variables|Default|GetWanderRadius) 0 0))))
        (AI|Navigation|SimpleMovetoLocation (Pawn|GetController) _output_get)))))

(fn SetCanWander
  (Variables|Default|SetCanWander true))

(fn InAttackRange
  (if (<= (Class|KismetMathLibrary|VectorDistanceSquared (Transformation|GetActorLocation) (Transformation|GetActorLocation (Game|Player|GetPlayerPawn 0))) (Variables|Default|GetAttackRange))
    (Variables|Default|SetAttacking true)
    (else
      (Variables|Default|SetAttacking false))))

(fn Attack
  (if (not (Variables|Default|GetIsFiring))
    (bind _returnvalue (Game|SpawnActorfromClass "/Game/Blueprints/Enemy_Actors/ConeAttack_2.ConeAttack_2_C" (Math|Transform|MakeTransform (Transformation|GetWorldLocation (Variables|Default|Getw)) (Math|Rotator|MakeRotator 0.0 0.0 (.yaw (Transformation|GetWorldRotation (Variables|Default|Getw)))) "1,1,1") "AdjustIfPossibleButAlwaysSpawn" 0 0))
    (Variables|Default|SetCurrentCone _returnvalue)
    (Variables|Default|SetIsFiring true)))

(fn SearchandDestroy
  (bind _returnvalue (Game|Player|GetPlayerPawn 0))
  (bind _returnvalue_2 (Transformation|GetActorLocation))
  (bind _returnvalue_3 (Utilities|Time|GetWorldDeltaSeconds))
  (bind _movespeed (Variables|Default|GetMoveSpeed))
  (bind _returnvalue_4 (Transformation|GetActorLocation _returnvalue))
  (bind _returnvalue_5 (* _movespeed _returnvalue_3))
  (bind _returnvalue_6 (- _returnvalue_4 _returnvalue_2))
  (bind _returnvalue_7 (Math|Vector|Normalize _returnvalue_6))
  (bind _returnvalue_8 (* _returnvalue_7 _returnvalue_5))
  (if (Variables|Default|GetAttacking)
    (if (not (Variables|Default|GetIsFiring))
      (Game|SpawnActorfromClass "/Game/Blueprints/Enemy_Actors/ConeAttack_2.ConeAttack_2_C" (Math|Transform|MakeTransform (Transformation|GetWorldLocation (Variables|Default|Getw)) (Math|Rotator|MakeRotator 0.0 0.0 (.yaw (Transformation|GetWorldRotation (Variables|Default|Getw)))) "1,1,1") "AdjustIfPossibleButAlwaysSpawn" 0 0)
      (Variables|Default|SetIsFiring true))
    (else
      (Transformation|AddActorWorldOffset (Math|Vector|MakeVector (.x _returnvalue_8) (.y _returnvalue_8) 0.0)))))