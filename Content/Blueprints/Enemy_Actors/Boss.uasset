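; Boss enemy that fires ranged attacks at the player, summons minions when hurt and prints a win message on death.
; BasicAttack and WaveAttack start at BeginPlay, firing single or five-point projectiles within squared-distance range; only their out-of-range branches set looping timers.
; While UsingRanged is set, Tick rotates the boss toward the player.
; AnyDamage reduces HP, triggers a one-time Bloat, Husk and Reaper spawn at low health, and destroys the boss at zero.
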(event EventBeginPlay
  (CallFunction|BasicAttack)
  (CallFunction|WaveAttack))

(event Collision|EventActorBeginOverlap
  (params (OtherActor :type Actor%20Object%20Reference)))

(event EventTick
  (params (DeltaSeconds :type Float%20%28single-precision%29))
  (if (Variables|Default|GetUsingRanged)
    (Transformation|SetActorRotation (Math|Rotator|MakeRotfromX (- (Transformation|GetActorLocation (Game|Player|GetPlayerPawn 0)) (Transformation|GetActorLocation))))))

(event Game|Damage|EventAnyDamage
  (params (Damage :type Float%20%28single-precision%29) (DamageType :type Damage%20Type%20Object%20Reference) (InstigatedBy :type Controller%20Object%20Reference) (DamageCauser :type Actor%20Object%20Reference))
  (bind _output_get (Variables|Default|SetHP (- (Variables|Default|GetHP) Damage)))
  (if (<= _output_get 5e+02)
    (CallFunction|CallHelp)
    (Variables|Default|SetHas%20called%20for%20Help true)
    (if (<= _output_get 0.0)
      (Actor|DestroyActor)
      (Development|PrintString "You WIN"))))

(fn ConstructionScript)

(fn WaveAttack
  (bind _waveattackpt1 (Variables|Default|GetWaveAttackPt1))
  (bind _waveattackpt2 (Variables|Default|GetWaveAttackPt2))
  (bind _waveattackpt3 (Variables|Default|GetWaveAttackPt3))
  (bind _waveattackpt4 (Variables|Default|GetWaveAttackPt4))
  (bind _waveattackpt5 (Variables|Default|GetWaveAttackPt5))
  (if (<= (Class|KismetMathLibrary|VectorDistanceSquared (Transformation|GetActorLocation) (Transformation|GetActorLocation (Game|Player|GetPlayerPawn 0))) (Variables|Default|GetRanged%20Attack%20Area))
    (Variables|Default|SetUsingRanged true)
    (Game|SpawnActorfromClass "/Game/Blueprints/Enemy_Actors/BossBullets.BossBullets_C" (Math|Transform|MakeTransform (Transformation|GetWorldLocation _waveattackpt1) (Transformation|GetWorldRotation _waveattackpt1) "1,1,1") "Undefined" 0 0)
    (Game|SpawnActorfromClass "/Game/Blueprints/Enemy_Actors/BossBullets.BossBullets_C" (Math|Transform|MakeTransform (Transformation|GetWorldLocation _waveattackpt2) (Transformation|GetWorldRotation _waveattackpt2) "1,1,1") "Undefined" 0 0)
    (Game|SpawnActorfromClass "/Game/Blueprints/Enemy_Actors/BossBullets.BossBullets_C" (Math|Transform|MakeTransform (Transformation|GetWorldLocation _waveattackpt3) (Transformation|GetWorldRotation _waveattackpt3) "1,1,1") "Undefined" 0 0)
    (Game|SpawnActorfromClass "/Game/Blueprints/Enemy_Actors/BossBullets.BossBullets_C" (Math|Transform|MakeTransform (Transformation|GetWorldLocation _waveattackpt4) (Transformation|GetWorldRotation _waveattackpt4) "1,1,1") "Undefined" 0 0)
    (Game|SpawnActorfromClass "/Game/Blueprints/Enemy_Actors/BossBullets.BossBullets_C" (Math|Transform|MakeTransform (Transformation|GetWorldLocation _waveattackpt5) (Transformation|GetWorldRotation _waveattackpt5) "1,1,1") "Undefined" 0 0)
    (else
      (Variables|Default|SetUsingRanged false)
      (Utilities|Time|SetTimerbyFunctionName 0 "WaveAttack" (Variables|Default|GetWave%20Attack%20Delay) true))))

(fn BasicAttack
  (bind _basicattack (Variables|Default|GetBasicAttack))
  (if (<= (Class|KismetMathLibrary|VectorDistanceSquared (Transformation|GetActorLocation) (Transformation|GetActorLocation (Game|Player|GetPlayerPawn 0))) (Variables|Default|GetRanged%20Attack%20Area))
    (Variables|Default|SetUsingRanged true)
    (Game|SpawnActorfromClass "/Game/Blueprints/Enemy_Actors/BossBulletVarient.BossBulletVarient_C" (Math|Transform|MakeTransform (Transformation|GetWorldLocation _basicattack) (Transformation|GetWorldRotation _basicattack) "1,1,1") "Undefined" 0 0)
    (else
      (Variables|Default|SetUsingRanged false)
      (Utilities|Time|SetTimerbyFunctionName 0 "Basic Attack" (Variables|Default|GetBasicAttackDelay) true))))

(fn CallHelp
  (bind _bloat_spawn_2 (Variables|Default|GetBloat%20Spawn%202))
  (bind _bloat_spawn_1 (Variables|Default|GetBloat%20Spawn%201))
  (bind _husk_spawn_2 (Variables|Default|GetHusk%20Spawn%202))
  (bind _husk_spawn_1 (Variables|Default|GetHusk%20Spawn%201))
  (bind _reaper_spawn (Variables|Default|GetReaper%20Spawn))
  (if (not (Variables|Default|GetHas%20called%20for%20Help))
    (Game|SpawnActorfromClass "/Game/Blueprints/Enemy_Actors/Bloat.Bloat_C" (Math|Transform|MakeTransform (Transformation|GetWorldLocation _bloat_spawn_1) (Transformation|GetWorldRotation _bloat_spawn_1) "1,1,1") "Undefined" 0 0)
    (Game|SpawnActorfromClass "/Game/Blueprints/Enemy_Actors/Bloat.Bloat_C" (Math|Transform|MakeTransform (Transformation|GetWorldLocation _bloat_spawn_2) (Transformation|GetWorldRotation _bloat_spawn_2) "1,1,1") "Undefined" 0 0)
    (Game|SpawnActorfromClass "/Game/Blueprints/Enemy_Actors/Husk.Husk_C" (Math|Transform|MakeTransform (Transformation|GetWorldLocation _husk_spawn_1) (Transformation|GetWorldRotation _husk_spawn_1) "1,1,1") "Undefined" 0 0)
    (Game|SpawnActorfromClass "/Game/Blueprints/Enemy_Actors/Husk.Husk_C" (Math|Transform|MakeTransform (Transformation|GetWorldLocation _husk_spawn_2) (Transformation|GetWorldRotation _husk_spawn_2) "1,1,1") "Undefined" 0 0)
    (Game|SpawnActorfromClass "/Game/Blueprints/Enemy_Actors/Reaper.Reaper_C" (Math|Transform|MakeTransform (Transformation|GetWorldLocation _reaper_spawn) (Transformation|GetWorldRotation _reaper_spawn) "1,1,1") "Undefined" 0 0)))