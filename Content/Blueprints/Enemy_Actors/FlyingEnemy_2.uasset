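; Flying enemy actor that chases and shoots at the player and destroys itself when it hits the MainCharacter.
; A FireRate-based timer runs SearchForPlayerAndFire, which checks squared distance, sets InRange and spawns StndEnemyBullet_2 at FirePT.
; The timer only becomes looping through the out-of-range branch.
; While InRange, Tick applies the normalized world direction to the player as a swept local offset and yaws toward them.
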(event EventBeginPlay
  (Utilities|Time|SetTimerbyFunctionName 0 "SearchForPlayerAndFire" (/ 1.0 (Variables|Default|GetFireRate))))

(event EventTick
  (params (DeltaSeconds :type Float%20%28single-precision%29))
  (if (Variables|Default|GetInRange)
    (Utilities|FlowControl|Sequence
      (:then_0
        (Transformation|AddActorLocalOffset (* (Math|Vector|Normalize (- (Transformation|GetActorLocation (Game|Player|GetPlayerPawn 0)) (Transformation|GetActorLocation))) (* (Variables|Default|GetMoveSpeed) (Utilities|Time|GetWorldDeltaSeconds))) true false))
      (:then_1
        (Transformation|SetActorRotation (Math|Rotator|MakeRotator 0.0 0.0 (.yaw (Math|Rotator|MakeRotfromX (- (Transformation|GetActorLocation (Game|Player|GetPlayerPawn 0)) (Transformation|GetActorLocation))))))))))

(event Collision|EventHit
  (params (MyComp :type Primitive%20Component%20Object%20Reference) (Other :type Actor%20Object%20Reference) (OtherComp :type Primitive%20Component%20Object%20Reference) (bSelfMoved :type Boolean) (HitLocation :type Vector :default "0, 0, 0") (HitNormal :type Vector :default "0, 0, 0") (NormalImpulse :type Vector :default "0, 0, 0") (Hit :type Hit%20Result%20Structure%20%28by%20ref%29))
  (Utilities|Casting|CastToMainCharacter Other)
  (Actor|DestroyActor))

(fn ConstructionScript)

(fn SearchforPlayerandFire
  (bind _firept (Variables|Default|GetFirePT))
  (if (<= (Class|KismetMathLibrary|VectorDistanceSquared (Transformation|GetActorLocation) (Transformation|GetActorLocation (Game|Player|GetPlayerPawn 0))) (Variables|Default|GetFireRangeSqur))
    (Variables|Default|SetInRange true)
    (Game|SpawnActorfromClass "/Game/Blueprints/Enemy_Actors/StndEnemyBullet_2.StndEnemyBullet_2_C" (Math|Transform|MakeTransform (Transformation|GetWorldLocation _firept) (Transformation|GetWorldRotation _firept) "1,1,1") "Undefined" 0 0)
    (else
      (Variables|Default|SetInRange false)
      (Utilities|Time|SetTimerbyFunctionName 0 "SearchForPlayerAndFire" (/ 1.0 (Variables|Default|GetFireRate)) true))))