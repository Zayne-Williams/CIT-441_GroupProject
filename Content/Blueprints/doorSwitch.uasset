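; Sliding door actor that the player opens with the interact button while standing inside its trigger box.
; When MainCharacter enters the box, the actor enables input and shows an EtoOpen prompt widget; leaving disables input and removes the prompt.
; Interacting plays the DoorOpen timeline, which drives the door mesh's relative location.
; Leaving the box reverses that timeline to close the door automatically.
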(event OnComponentBeginOverlap(Box)
  (params (OverlappedComponent :type Primitive%20Component%20Object%20Reference) (OtherActor :type Actor%20Object%20Reference) (OtherComp :type Primitive%20Component%20Object%20Reference) (OtherBodyIndex :type Integer) (bFromSweep :type Boolean) (SweepResult :type Hit%20Result%20Structure%20%28by%20ref%29))
  ;[1 1 1] Jacob: Door mechanic that opens when a player presses activate within the trigger zone
  (Utilities|Casting|CastToMainCharacter OtherActor)
  (Input|EnableInput (Game|GetPlayerController 0))
  (bind _returnvalue (UserInterface|CreateWidget "/Game/Blueprints/EtoOpen.EtoOpen_C"))
  (bind _output_get (Variables|Default|SetEtoOpen _returnvalue))
  (UserInterface|Viewport|AddtoViewport _output_get 0))

(event OnComponentEndOverlap(Box)
  (params (OverlappedComponent :type Primitive%20Component%20Object%20Reference) (OtherActor :type Actor%20Object%20Reference) (OtherComp :type Primitive%20Component%20Object%20Reference) (OtherBodyIndex :type Integer))
  ;[1 1 1] Jacob: Door mechanic that opens when a player presses activate within the trigger zone
  (Utilities|Casting|CastToMainCharacter OtherActor)
  (Input|DisableInput (Game|GetPlayerController 0))
  (Widget|RemovefromParent (Variables|Default|GetEtoOpen))
  (bind _slide_of_the_door (Timeline|Door%20Open Reverse)
    (:Update
      (Transformation|SetRelativeLocation (Variables|Default|GetDoorMesh) _slide_of_the_door false false))))

(event EventBeginPlay)

(event Collision|EventActorBeginOverlap
  (params (OtherActor :type Actor%20Object%20Reference)))

(event EventTick
  (params (DeltaSeconds :type Float%20%28single-precision%29)))

(event Input|ActionEvents|InputActionInteractButton
  (params (Key :type Key%20Structure :default "None"))
  ;[1 1 1] Jacob: Door mechanic that opens when a player presses activate within the trigger zone
  (:Pressed
    (bind _slide_of_the_door (Timeline|Door%20Open Play)
      (:Update
        (Transformation|SetRelativeLocation (Variables|Default|GetDoorMesh) _slide_of_the_door false false)))))

(fn ConstructionScript)