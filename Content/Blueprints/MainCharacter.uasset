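; First-person player character handling movement, shooting, bullet time, inventory, interaction, pause and death.
; BeginPlay builds HUD widgets, attaches the weapon to the arms socket and restores health and position from a save slot.
; Weapon switching cycles five classes by respawning the actor; firing aims via a camera line trace that requires a hitscan weapon.
; Tick sphere-traces for hover messages and teleports fallen players to the level start.
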(event EventTick
  (params (DeltaSeconds :type Float%20%28single-precision%29))
  (bind _camera (Variables|Default|GetCamera))
  (bind _returnvalue (Transformation|GetWorldLocation _camera))
  ;[1 1 1] Asad Ranavaya
  ;;[1 1 1] Interact, Hover and unhover
  (CallFunction|CheckifFall)
  (bind (_outhit _returnvalue_2) (Collision|SphereTraceByChannel _returnvalue (+ _returnvalue (* (Math|Vector|GetForwardVector _camera) 250)) 0.0 "TraceTypeQuery1" false 0 "None"))
  (if _returnvalue_2
    (if (!= (Variables|Default|GetTracedObject) (.hitactor _outhit))
      (Class|InteractInterface|Unhover(Message) (Variables|Default|GetTracedObject))
      (bind _output_get (Variables|Default|SetTracedObject (.hitactor _outhit)))
      (Class|InteractInterface|Hover(Message) _output_get))
    (else
      (Utilities|IsValid (Variables|Default|GetTracedObject)
        (:Is%20Valid
          (Class|InteractInterface|Unhover(Message) (Variables|Default|GetTracedObject))
          (Variables|Default|SetTracedObject 0))))))

(event EventBeginPlay
  ;[1 1 1] Andrew
  ;[1 1 1] Comment
  (AddComponent|AddAudioComponent false)
  (Variables|Default|SetlevelStartingPos (Transformation|GetActorLocation))
  (bind _returnvalue (UserInterface|CreateWidget "/Game/UI/Respects.Respects_C"))
  (bind _output_get (Variables|Default|SetRespect%20Widget _returnvalue))
  (UserInterface|Viewport|AddtoViewport _output_get 0)
  (Widget|SetVisibility (Variables|Default|GetRespect%20Widget) "Hidden")
  (bind _returnvalue_2 (Game|SpawnActorfromClass (Variables|Default|GetWeaponClass) (Transformation|GetSocketTransform (Variables|Default|GetArms%20Mesh) "R_GunSocket" "RTS_World") "Undefined" 0 0))
  (bind _output_get_2 (Variables|Default|SetCurrentWeapon _returnvalue_2))
  (Class|SkinnedMeshComponent|SetSkeletalMesh (Variables|/Game/WeaponStuff/BP_BaseWeapon.BP_BaseWeapon_C|GetGunMesh _output_get_2) (Variables|/Script/Engine.SkinnedMeshComponent|GetSkeletalMesh (Variables|/Game/WeaponStuff/BP_BaseWeapon.BP_BaseWeapon_C|GetGunMesh (Variables|Default|GetCurrentWeapon))) true)
  (Transformation|AttachComponentToComponent _output_get_2 (Variables|Default|GetArms%20Mesh) "R_GunSocket" "SnapToTarget" "SnapToTarget" "KeepWorld" true)
  ;[1 1 1] Comment
  (bind _returnvalue_3 (UserInterface|CreateWidget "/Game/UI/HealthHUD.HealthHUD_C"))
  (Progress|SetPercent (Variables|/Game/UI/HealthHUD.HealthHUD_C|GethealthBar _returnvalue_3) (Variables|Default|GetcurrentHealth))
  (UserInterface|Viewport|AddtoViewport _returnvalue_3 0)
  (bind _returnvalue_4 (SaveGame|DoesSaveGameExist "Save1"))
  (if _returnvalue_4
    (bind _returnvalue_5 (SaveGame|LoadGamefromSlot "Save1"))
    (bind _ascorona_save_game (Utilities|Casting|CastToCoronaSaveGame _returnvalue_5))
    (Variables|Default|SetcurrentHealth (Variables|/Game/Blueprints/CoronaSaveGame.CoronaSaveGame_C|GetHealth _ascorona_save_game))
    (if (Variables|/Game/Blueprints/CoronaSaveGame.CoronaSaveGame_C|GetisNewLevel _ascorona_save_game)
      (Variables|/Game/Blueprints/CoronaSaveGame.CoronaSaveGame_C|SetisNewLevel _ascorona_save_game false)
      (SaveGame|SaveGametoSlot _ascorona_save_game "Save1")
      (Transformation|SetActorLocation "-7942.000000, 0,474.000000" false false)
      (else
        (Transformation|SetActorLocation (Variables|/Game/Blueprints/CoronaSaveGame.CoronaSaveGame_C|GetplayersLastPosition _ascorona_save_game) false false)))
    (else
      (bind _returnvalue_6 (SaveGame|CreateSaveGameObject "/Game/Blueprints/CoronaSaveGame.CoronaSaveGame_C"))
      (SaveGame|SaveGametoSlot _returnvalue_6 "Save1"))))

(event Input|ActionEvents|InputActionCrouch
  (params (Key :type Key%20Structure :default "None"))
  ;[1 1 1] Asad Ranavaya
  ;;[1 1 1] Movement
  (:Pressed
    (Character|Crouch))
  (:Released
    (Character|UnCrouch)))

(event Input|ActionEvents|InputActionJump
  (params (Key :type Key%20Structure :default "None"))
  ;[1 1 1] Asad Ranavaya
  ;;[1 1 1] Movement
  (:Pressed
    (Character|Jump))
  (:Released
    (Character|StopJumping)))

(event Input|ActionEvents|InputActionPauseGame
  (params (Key :type Key%20Structure :default "None"))
  ;[1 1 1] Asad Ranavaya
  ;;[1 1 1] Pause Game
  (:Pressed
    (Game|SetGamePaused true)
    (bind _returnvalue (UserInterface|CreateWidget "/Game/UI/PauseGame.PauseGame_C"))
    (UserInterface|Viewport|AddtoViewport _returnvalue 0)
    (bind _asmain_character_controller (Utilities|Casting|CastToMainCharacterController (Game|GetPlayerController 0)))
    (Variables|/Script/Engine.PlayerController|SetbShowMouseCursor _asmain_character_controller true)))

(event Input|ActionEvents|InputActionInteractButton
  (params (Key :type Key%20Structure :default "None"))
  (bind _widgetinteraction (Variables|Default|GetWidgetInteraction))
  ;[1 1 1] Asad Ranavaya
  ;;[1 1 1] Interact with world widget
  (:Pressed
    (Class|WidgetInteractionComponent|PressPointerKey _widgetinteraction "LeftMouseButton")
    (Class|WidgetInteractionComponent|ReleasePointerKey _widgetinteraction "LeftMouseButton")))

(event Input|ActionEvents|InputActionSprint
  (params (Key :type Key%20Structure :default "None"))
  (bind _charactermovement (Variables|Character|GetCharacterMovement))
  ;[1 1 1] Asad Ranavaya
  ;;[1 1 1] Movement
  (:Pressed
    (bind _output_get (Variables|/Script/Engine.CharacterMovementComponent|SetMaxWalkSpeed _charactermovement (* (Class|MovementComponent|GetMaxSpeed _charactermovement) 2.0))))
  (:Released
    (Variables|/Script/Engine.CharacterMovementComponent|SetMaxWalkSpeed _charactermovement (/ _output_get 2.0))))

(event Input|ActionEvents|InputActionPayRespects
  (params (Key :type Key%20Structure :default "None"))
  (bind _respect_widget (Variables|Default|GetRespect%20Widget))
  ;[1 1 1] Asad Ranavaya
  ;;[1 1 1] Press F
  (:Pressed
    (Widget|SetVisibility _respect_widget "Visible"))
  (:Released
    (Utilities|FlowControl|Delay 1.0)
    (Widget|SetVisibility _respect_widget "Hidden")))

(event Input|ActionEvents|InputActionInteractButton
  (params (Key :type Key%20Structure :default "None"))
  ;[1 1 1] Asad Ranavaya
  ;;[1 1 1] Inventory System
  (:Pressed
    (bind _array_element (Utilities|Array|ForEachLoopwithBreak (Collision|GetOverlappingActors "/Script/Engine.Actor" :!class /Script/Engine.Actor) :!label _label)
      (:LoopBody
        (if (Utilities|DoesObjectImplementInterface _array_element "/Game/InventorySystem/Interact_Interface.Interact_Interface_C")
          (Class|InteractInterface|Interact(Message) _array_element self)
          (goto _label Break))))))

(event Input|ActionEvents|InputActionInventory
  (params (Key :type Key%20Structure :default "None"))
  ;[1 1 1] Asad Ranavaya
  ;;[1 1 1] Inventory System
  (:Pressed
    (Default|ToggleInventory (Variables|Default|GetInventoryComponent))))

(event Input|ActionEvents|InputActionFireWeapon
  (params (Key :type Key%20Structure :default "None"))
  (bind _currentweapon (Variables|Default|GetCurrentWeapon))
  (bind _arms_mesh (Variables|Default|GetArms%20Mesh))
  (bind _returnvalue (Components|SkeletalMesh|GetAnimInstance _arms_mesh))
  ;[1 1 1] Andrew
  (:Pressed
    (Utilities|IsValid _currentweapon
      (:Is%20Valid
        (bind _crosshairworldspace (CallFunction|GetCrosshairWorldspace))
        (Default|Fire _currentweapon _crosshairworldspace)
        (if (== (Math|Random|RandomIntegerinRange 1 2) 1)
          (Animation|Montage|MontagePlay _returnvalue "/Game/WeaponStuff/FPS_Assault_Pack/Animations/RU74/A_Arms_RU74_Shoot01_Montage.A_Arms_RU74_Shoot01_Montage" 1.0 "MontageLength" 0.0 true)
          (else
            (Animation|Montage|MontagePlay _returnvalue "/Game/WeaponStuff/FPS_Assault_Pack/Animations/RU74/A_Arms_RU74_Shoot02_Montage.A_Arms_RU74_Shoot02_Montage" 1.0 "MontageLength" 0.0 true)))))))

(event Input|ActionEvents|InputActionSwitchWeapon
  (params (Key :type Key%20Structure :default "None"))
  ;[1 1 1] Andrew
  ;;[1 1 1] Switch Weapon
  (:Pressed
    (Actor|DestroyActor (Variables|Default|GetCurrentWeapon))
    (switch int (Variables|Default|GetWeaponNum)
      (:0
        (Variables|Default|SetWeaponClass "/Game/WeaponStuff/BP_Shotgun.BP_Shotgun_C")
        (Variables|Default|SetWeaponNum 1))
      (:1
        (Variables|Default|SetWeaponClass "/Game/WeaponStuff/BP_AssultRifle.BP_AssultRifle_C")
        (Variables|Default|SetWeaponNum 2))
      (:2
        (Variables|Default|SetWeaponClass "/Game/WeaponStuff/BP_GrenadeLauncher.BP_GrenadeLauncher_C")
        (Variables|Default|SetWeaponNum 3))
      (:3
        (Variables|Default|SetWeaponClass "/Game/WeaponStuff/BP_RocketLauncher.BP_RocketLauncher_C")
        (Variables|Default|SetWeaponNum 4))
      (:4
        (Variables|Default|SetWeaponClass "/Game/WeaponStuff/BP_Pistol.BP_Pistol_C")
        (Variables|Default|SetWeaponNum 0)))
    (bind _returnvalue (Game|SpawnActorfromClass (Variables|Default|GetWeaponClass) (Transformation|GetSocketTransform (Variables|Default|GetArms%20Mesh) "R_GunSocket" "RTS_World") "Undefined" 0 0))
    (bind _output_get (Variables|Default|SetCurrentWeapon _returnvalue))
    (Class|SkinnedMeshComponent|SetSkeletalMesh (Variables|/Game/WeaponStuff/BP_BaseWeapon.BP_BaseWeapon_C|GetGunMesh _output_get) (Variables|/Script/Engine.SkinnedMeshComponent|GetSkeletalMesh (Variables|/Game/WeaponStuff/BP_BaseWeapon.BP_BaseWeapon_C|GetGunMesh (Variables|Default|GetCurrentWeapon))) true)
    (Transformation|AttachComponentToComponent _output_get (Variables|Default|GetArms%20Mesh) "R_GunSocket" "SnapToTarget" "SnapToTarget" "KeepWorld" true)))

(event Input|ActionEvents|InputActionBulletTime
  (params (Key :type Key%20Structure :default "None"))
  ;[1 1 1] Andrew
  (:Pressed
    (Variables|Default|SetisSlomo true)
    (Utilities|Time|SetGlobalTimeDilation 0.12))
  (:Released
    (Variables|Default|SetisSlomo false)
    (Utilities|Time|SetGlobalTimeDilation 1.0)))

(event Input|ActionEvents|InputActionReload
  (params (Key :type Key%20Structure :default "None"))
  (bind _currentweapon (Variables|Default|GetCurrentWeapon))
  ;[1 1 1] Andrew
  (:Pressed
    (Utilities|IsValid _currentweapon
      (:Is%20Valid
        (Default|Reload _currentweapon)
        (Animation|Montage|MontagePlay (Components|SkeletalMesh|GetAnimInstance (Variables|Default|GetArms%20Mesh)) "/Game/WeaponStuff/FPS_Assault_Pack/Animations/RU74/A_Arms_RU74_Reload_Montage.A_Arms_RU74_Reload_Montage" 1.0 "MontageLength" 0.1 true)))))

(event Input|AxisEvents|InputAxisMoveFront/Back
  (params (AxisValue :type Float%20%28single-precision%29))
  ;[1 1 1] Asad Ranavaya
  ;;[1 1 1] Movement
  (Class|PawnMovementComponent|AddInputVector (Variables|Character|GetCharacterMovement) (* (Transformation|GetActorForwardVector) AxisValue) false))

(event Input|AxisEvents|InputAxisMoveSide
  (params (AxisValue :type Float%20%28single-precision%29))
  ;[1 1 1] Asad Ranavaya
  ;;[1 1 1] Movement
  (Class|PawnMovementComponent|AddInputVector (Variables|Character|GetCharacterMovement) (* (Transformation|GetActorRightVector) AxisValue) false))

(event Input|AxisEvents|InputAxisLookVertical
  (params (AxisValue :type Float%20%28single-precision%29))
  ;[1 1 1] Asad Ranavaya
  ;;[1 1 1] Movement
  (Pawn|Input|AddControllerPitchInput (* AxisValue -1.0))
  (Transformation|AddLocalRotation (Variables|Character|GetMesh) (Math|Rotator|MakeRotator 0.0 (* 2 AxisValue) 0.0) false false))

(event Input|AxisEvents|InputAxisLookSide
  (params (AxisValue :type Float%20%28single-precision%29))
  ;[1 1 1] Asad Ranavaya
  ;;[1 1 1] Movement
  (Pawn|Input|AddControllerYawInput AxisValue))

(event Input|KeyboardEvents|Q
  (params (Key :type Key%20Structure :default "None"))
  ;[1 1 1] Asad Ranavaya
  ;;[1 1 1] Test Query of Inventory
  (:Pressed
    (bind _isininventory (Default|InventoryQuery (Variables|Default|GetInventoryComponent) "/Game/InventorySystem/Item/Item_Block.Item_Block_C" 1))
    (if _isininventory
      (Development|PrintString "Item Found")
      (else
        (Development|PrintString "Not Found :/")))))

(fn ConstructionScript)

(fn GetCrosshairWorldspace
  (bind _camera (Variables|Default|GetCamera))
  (bind _returnvalue (Transformation|GetWorldLocation _camera))
  (bind _asbp_hitscan_weapon (Utilities|Casting|CastToBP_HitscanWeapon (Variables|Default|GetCurrentWeapon)))
  (bind (_outhit _returnvalue_2) (Collision|LineTraceByChannel _returnvalue (+ _returnvalue (* (Math|Rotator|GetRotationXVector (Pawn|GetBaseAimRotation self)) (Variables|/Game/WeaponStuff/BP_HitscanWeapon.BP_HitscanWeapon_C|GetRange _asbp_hitscan_weapon))) "TraceTypeQuery1" false 0 "None"))
  (if _returnvalue_2
    (Development|PrintString "InLineTraceTrue")
    (return (.location _outhit))
    (else
      (Development|PrintString "InLineTraceFalse")
      (return (+ _returnvalue (* (Math|Rotator|GetRotationXVector (Pawn|GetBaseAimRotation self)) (Variables|/Game/WeaponStuff/BP_HitscanWeapon.BP_HitscanWeapon_C|GetRange _asbp_hitscan_weapon)))))))

(fn DecrementHealth
  (params (Difference :type Float%20%28single-precision%29))
  (Variables|Default|SetcurrentHealth (Math|Float|Clamp(Float) (- (Variables|Default|GetcurrentHealth) Difference) 0.0 (Variables|Default|GetMaxHealth)))
  (if (<= (Variables|Default|GetcurrentHealth) 0.001)
    (CallFunction|CheckHealth)))

(fn CheckHealth
  (if (<= (Variables|Default|GetcurrentHealth) 0.0)
    (bind _returnvalue (UserInterface|CreateWidget "/Game/UI/DeathScreen.DeathScreen_C"))
    (UserInterface|Viewport|AddtoViewport _returnvalue 0)
    (bind _asmain_character_controller (Utilities|Casting|CastToMainCharacterController (Game|GetPlayerController 0)))
    (Variables|/Script/Engine.PlayerController|SetbShowMouseCursor _asmain_character_controller true)
    (Input|DisableInput _asmain_character_controller)
    (Game|SetGamePaused true)))

(fn CheckifFall
  (if (<= (.z (Transformation|GetActorLocation)) -5e+02)
    (Transformation|SetActorLocation (Variables|Default|GetlevelStartingPos) false false)))